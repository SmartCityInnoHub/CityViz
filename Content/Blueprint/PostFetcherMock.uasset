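; PostFetcherMock is an actor that stands in for a post fetcher by feeding random canned posts into a PostFeeder.
; On BeginPlay it starts a looping timer with an interval randomized once between 3 and 3.5 seconds.
; Each tick of the timer adds a random Textpool entry to the feeder's PostChannel and logs the returned index with a separately drawn random entry.
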(event EventBeginPlay
  (Utilities|Time|SetTimerbyFunctionName self "GenerateNewPost" (+ (* (Math|Random|RandomFloat) 0.5) 3.0) true))

(event Collision|EventActorBeginOverlap
  (params (OtherActor :type Actor%20Object%20Reference)))

(event EventTick
  (params (DeltaSeconds :type Float%20%28single-precision%29)))

(fn ConstructionScript)

(fn GenerateNewPost
  (bind _textpool (LocalVariables|Gettextpool))
  (bind _returnvalue (Utilities|Array|Length _textpool))
  (bind _returnvalue_2 (Math|Random|RandomInteger _returnvalue))
  (bind _output (Utilities|Array|Get(acopy) _textpool _returnvalue_2))
  (bind _returnvalue_3 (Utilities|Array|Add (Variables|/Script/CityViz.PostFeeder|GetPostChannel (Variables|Default|GetPostFeeder)) _output))
  (Class|VisualLoggerKismetLibrary|LogText (Utilities|String|Append (Utilities|String|ToString(Integer) _returnvalue_3) " At " _output) "Blueprint Log"))